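; Player forklift on Chaos vehicle physics that picks up and throws crates, with most tuning read from a DataAsset.
; Crates overlapping both detection boxes attach to the fork, whose height timeline also sets throw angle, and charged launches scale with hold time.
; Boost adds steering-biased force with exhaust VFX, then recharges by timer once depleted.
; It also handles camera auto-rotation behind the vehicle, checkpoint respawn and the pause menu.
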(event OnComponentBeginOverlap(boxDetection)
  (params (OverlappedComponent :type Primitive%20Component%20Object%20Reference) (OtherActor :type Actor%20Object%20Reference) (OtherComp :type Primitive%20Component%20Object%20Reference) (OtherBodyIndex :type Integer) (bFromSweep :type Boolean) (SweepResult :type Hit%20Result%20Structure%20%28by%20ref%29))
  (bind _boxdetection (Variables|Default|GetboxDetection))
  (bind _crateloc (Variables|Default|GetCrateLoc))
  (bind _overlappingactors (Collision|GetOverlappingActors _boxdetection 0 :!class /Script/Engine.PrimitiveComponent))
  (bind _output (Utilities|Array|Get(acopy) _overlappingactors))
  ;[1 1 1] DetectCrate
  (Utilities|IsValid (Variables|Default|GetactualCrate)
    (:Is%20Not%20Valid
      (if (== _output (Utilities|Array|Get(acopy) (Collision|GetOverlappingActors (Variables|Default|GetboxDetection1) 0 :!class /Script/Engine.PrimitiveComponent)))
        (bind _output_get (Variables|Default|SetactualCrate _output))
        (Utilities|IsValid _output_get
          (:Is%20Valid
            (Class|BPIPickable|ChangePhysic(Message) _output_get false self)
            (Transformation|AttachComponentToComponent _output_get (Variables|Default|GetCrateLoc) "None" "KeepWorld" "KeepWorld" "KeepWorld" true)
            (Utilities|FlowControl|Delay 0.2)
            (bind _alpha (Timeline|MoveBoxToLoc PlayFromStart)
              (:Update
                (Transformation|SetActorLocationAndRotation (Variables|Default|GetactualCrate) (Math|Vector|Lerp(Vector) (Transformation|GetActorLocation (Variables|Default|GetactualCrate)) (Transformation|GetWorldLocation _crateloc) _alpha) (Math|Rotator|Lerp(Rotator) (Transformation|GetActorRotation (Variables|Default|GetactualCrate)) (Transformation|GetWorldRotation _crateloc) _alpha true)))
              (:Finished
                (bind _ashud_game (Utilities|Casting|CastToHUD_Game (HUD|GetHUD (Game|GetPlayerController 0))))
                (Default|LaunchPopUp (Variables|/Game/_Manager/InGame/HUD_Game.HUD_Game_C|GetWBP_PopUp _ashud_game))))))))))

(event OnComponentBeginOverlap(boxDetection1)
  (params (OverlappedComponent :type Primitive%20Component%20Object%20Reference) (OtherActor :type Actor%20Object%20Reference) (OtherComp :type Primitive%20Component%20Object%20Reference) (OtherBodyIndex :type Integer) (bFromSweep :type Boolean) (SweepResult :type Hit%20Result%20Structure%20%28by%20ref%29))
  (bind _boxdetection (Variables|Default|GetboxDetection))
  (bind _crateloc (Variables|Default|GetCrateLoc))
  (bind _overlappingactors (Collision|GetOverlappingActors _boxdetection 0 :!class /Script/Engine.PrimitiveComponent))
  (bind _output (Utilities|Array|Get(acopy) _overlappingactors))
  ;[1 1 1] DetectCrate
  (Utilities|IsValid (Variables|Default|GetactualCrate)
    (:Is%20Not%20Valid
      (if (== _output (Utilities|Array|Get(acopy) (Collision|GetOverlappingActors (Variables|Default|GetboxDetection1) 0 :!class /Script/Engine.PrimitiveComponent)))
        (bind _output_get (Variables|Default|SetactualCrate _output))
        (Utilities|IsValid _output_get
          (:Is%20Valid
            (Class|BPIPickable|ChangePhysic(Message) _output_get false self)
            (Transformation|AttachComponentToComponent _output_get (Variables|Default|GetCrateLoc) "None" "KeepWorld" "KeepWorld" "KeepWorld" true)
            (Utilities|FlowControl|Delay 0.2)
            (bind _alpha (Timeline|MoveBoxToLoc PlayFromStart)
              (:Update
                (Transformation|SetActorLocationAndRotation (Variables|Default|GetactualCrate) (Math|Vector|Lerp(Vector) (Transformation|GetActorLocation (Variables|Default|GetactualCrate)) (Transformation|GetWorldLocation _crateloc) _alpha) (Math|Rotator|Lerp(Rotator) (Transformation|GetActorRotation (Variables|Default|GetactualCrate)) (Transformation|GetWorldRotation _crateloc) _alpha true)))
              (:Finished
                (bind _ashud_game (Utilities|Casting|CastToHUD_Game (HUD|GetHUD (Game|GetPlayerController 0))))
                (Default|LaunchPopUp (Variables|/Game/_Manager/InGame/HUD_Game.HUD_Game_C|GetWBP_PopUp _ashud_game))))))))))

(event Custom|RotateCam
  (bind _returnvalue (Game|GetPlayerController 0))
  (bind _returnvalue_2 (Pawn|GetControlRotation _returnvalue :!class /Script/Engine.Controller))
  (bind (_roll _pitch) (Math|Rotator|BreakRotator _returnvalue_2))
  ;[1 1 1] Look
  (Pawn|SetControlRotation _returnvalue (Math|Interpolation|RInterpTo _returnvalue_2 (Math|Rotator|MakeRotator _roll _pitch (.yaw (Transformation|GetActorRotation))) 0.001 (* (Variables|/Game/_Manager/InGame/DataAsset/BP/BP_Player_DA.BP_Player_DA_C|GetcameraAutoRotSpeed (Variables|Default|GetdataAsset)) (Math|Float|Clamp(Float) (/ (Math|Vector|VectorLength (Transformation|GetVelocity)) 3e+01) 0.0001 1e+01)))))

(event Custom|RecoverBoost
  ;[1 1 1] BoostRecover
  (bind _output_get (Variables|Default|SetBoostUsage (- (Variables|Default|GetBoostUsage) (* 1.0 (Utilities|Time|GetWorldDeltaSeconds)))))
  (if (<= _output_get 0.0)
    (Variables|Default|SetBoostUsage 0.0)
    (Variables|Default|SetbCanBoost true)
    (Utilities|Time|PauseTimerbyHandle (Variables|Default|GetboostRecoverHandle))
    (Development|PrintString "Boost recover")))

(event Custom|UnlinkBox_1
  (Variables|Default|SetactualCrate 0))

(event EventChargeBox
  (params (time :type Float%20%28double-precision%29))
  (bind _dataasset (Variables|Default|GetdataAsset))
  (bind _throwarrow (Variables|Default|GetthrowArrow))
  (bind _launchholdtime (Variables|/Game/_Manager/InGame/DataAsset/BP/BP_Player_DA.BP_Player_DA_C|GetlaunchHoldTime _dataasset))
  ;[1 1 1] LaunchBox
  (Utilities|IsValid (Variables|Default|GetactualCrate)
    (:Is%20Valid
      (bind _output_get (Variables|Default|SetlaunchStrength (+ (Utilities|Time|GetWorldDeltaSeconds) (Variables|Default|GetlaunchStrength))))
      (if (> _output_get _launchholdtime)
        (Utilities|FlowControl|Delay (Variables|/Game/_Manager/InGame/DataAsset/BP/BP_Player_DA.BP_Player_DA_C|GettimeBeforeReset (Variables|Default|GetdataAsset)))
        (Variables|Default|SetlaunchStrength 0.0)
        (else
          (Variables|/Script/Engine.ArrowComponent|SetArrowLength _throwarrow (Math|Float|Lerp 2e+01 4e+01 (/ (Variables|Default|GetlaunchStrength) _launchholdtime)))
          (Development|SetHiddeninGame _throwarrow (<= (Math|Float|Lerp 2e+01 4e+01 (/ (Variables|Default|GetlaunchStrength) _launchholdtime)) 0.1) false)
          (Default|SetWidgetVisibility (Variables|Default|GetchargeWidgetRef) true))))))

(event EventBoost
  (params (Activated :type Boolean))
  (bind _returnvalue (CallFunction|DesiredRotation))
  (bind _dataasset (Variables|Default|GetdataAsset))
  (bind _boostacceleration (Variables|/Game/_Manager/InGame/DataAsset/BP/BP_Player_DA.BP_Player_DA_C|GetboostAcceleration _dataasset))
  ;[1 1 1] Boost
  (if (Variables|Default|GetbCanBoost)
    (CallFunction|SetExhaustVFX Activated)
    (bind _output_get (Variables|Default|SetBoostUsage (+ (Variables|Default|GetBoostUsage) (* 1.0 (Utilities|Time|GetWorldDeltaSeconds)))))
    (Development|PrintString (Utilities|String|ToString(Float) _output_get) true true "(R=0.000000,G=0.660000,B=1.000000,A=1.000000)" 2.0 "Boost Usage")
    (if (< (Vehicle|GetForwardSpeed (Variables|Default|GetVehicleMovementComponent)) (Variables|/Game/_Manager/InGame/DataAsset/BP/BP_Player_DA.BP_Player_DA_C|GetboostSpeedLimit (Variables|Default|GetdataAsset)))
      (Physics|AddForce (Variables|Character|GetMesh) (Math|Vector|MakeVector (* (.x _returnvalue) _boostacceleration) (* (.y _returnvalue) _boostacceleration) 0.0) "None" true)
      (if (>= (Variables|Default|GetBoostUsage) (Variables|/Game/_Manager/InGame/DataAsset/BP/BP_Player_DA.BP_Player_DA_C|GetboostSpeedDuration (Variables|Default|GetdataAsset)))
        (Variables|Default|SetbCanBoost false)
        (bind _returnvalue_2 (Utilities|Time|SetTimerbyEvent (delegate Custom|RecoverBoost) 0.001 true true))
        (Variables|Default|SetboostRecoverHandle _returnvalue_2)))
    (else
      (CallFunction|SetExhaustVFX false))))

(event EventBeginPlay
  (bind _dataasset (Variables|Default|GetdataAsset))
  (bind _dataasset_2 (Variables|Default|GetdataAsset))
  (bind _springarm (Variables|Default|GetSpringArm))
  (bind _dataasset_3 (Variables|Default|GetdataAsset))
  (bind _camerabaselocation (Variables|/Game/_Manager/InGame/DataAsset/BP/BP_Player_DA.BP_Player_DA_C|GetcameraBaseLocation _dataasset))
  (bind _cameralag (Variables|/Game/_Manager/InGame/DataAsset/BP/BP_Player_DA.BP_Player_DA_C|GetcameraLag _dataasset_3))
  (bind _camerarotationlag (Variables|/Game/_Manager/InGame/DataAsset/BP/BP_Player_DA.BP_Player_DA_C|GetcameraRotationLag _dataasset_3))
  ;[1 1 1] Set DataAsset
  (CallFunction|SetupCameraAssets)
  (bind _aschaos_wheeled_vehicle_movement_component (Utilities|Casting|CastToChaosWheeledVehicleMovementComponent (Variables|Default|GetVehicleMovementComponent)))
  (Class|ChaosWheeledVehicleMovementComponent|SetMaxEngineTorque _aschaos_wheeled_vehicle_movement_component (Variables|/Game/_Manager/InGame/DataAsset/BP/BP_Player_DA.BP_Player_DA_C|GetmaxTorque _dataasset_2))
  (Class|ChaosWheeledVehicleMovementComponent|SetDifferentialFrontRearSplit _aschaos_wheeled_vehicle_movement_component (Variables|/Game/_Manager/InGame/DataAsset/BP/BP_Player_DA.BP_Player_DA_C|GetdifferentialFrontRearSplit _dataasset_2))
  (Components|Timeline|SetPlayRate (Variables|Default|GetforkLoc) (Variables|/Game/_Manager/InGame/DataAsset/BP/BP_Player_DA.BP_Player_DA_C|GetforkLiftingSpeed (Variables|Default|GetdataAsset)))
  (Variables|Throw|SetthrowAngle (Variables|/Game/_Manager/InGame/DataAsset/BP/BP_Player_DA.BP_Player_DA_C|GetlaunchingAngleMin (Variables|Default|GetdataAsset)))
  (Transformation|SetRelativeRotation (Variables|Default|GetthrowArrow) (Math|Rotator|MakeRotator 0.0 (Variables|Throw|GetthrowAngle) 0.0) false false)
  (Pawn|SetControlRotation (Game|GetPlayerController 0) (Math|Rotator|MakeRotator 0.0 (.x _camerabaselocation) (.y _camerabaselocation)))
  (Transformation|SetRelativeLocation (Variables|Default|GetSpringArm) (Variables|/Game/_Manager/InGame/DataAsset/BP/BP_Player_DA.BP_Player_DA_C|GetspringArmOffset (Variables|Default|GetdataAsset)) false false)
  (bind _foundwidgets (Widget|GetAllWidgetsOfClass "/Game/Blueprints/UI/WBP_Charge.WBP_Charge_C" false))
  (Variables|Default|SetchargeWidgetRef (Utilities|Array|Get(acopy) _foundwidgets))
  (Variables|Default|SetcheckpointTransform (Transformation|GetActorTransform))
  (Variables|/Script/Engine.SpringArmComponent|SetbEnableCameraLag _springarm (> _cameralag 0.0))
  (Variables|/Script/Engine.SpringArmComponent|SetCameraLagSpeed _springarm _cameralag)
  (Variables|/Script/Engine.SpringArmComponent|SetbEnableCameraRotationLag _springarm (> _camerarotationlag 0.0))
  (Variables|/Script/Engine.SpringArmComponent|SetCameraRotationLagSpeed _springarm _camerarotationlag)
  (Transformation|SetRelativeLocation (Variables|Default|GetSpringArm) (Variables|/Game/_Manager/InGame/DataAsset/BP/BP_Player_DA.BP_Player_DA_C|GetspringArmOffset (Variables|Default|GetdataAsset)) false false))

(event EventLaunchBox
  ;[1 1 1] LaunchBox
  (if (and (Utilities|IsValid (Variables|Default|GetactualCrate)) (> (Variables|Default|GetlaunchStrength) (Variables|/Game/_Manager/InGame/DataAsset/BP/BP_Player_DA.BP_Player_DA_C|GetlaunchHoldMin (Variables|Default|GetdataAsset))))
    (Development|SetHiddeninGame (Variables|Default|GetthrowArrow) true false)
    (Default|PlayThrowAimation (Variables|Default|GetchargeWidgetRef))
    (Components|Activation|SetActive (Variables|Default|GetboxDetection) false false)
    (Components|Activation|SetActive (Variables|Default|GetboxDetection1) false false)
    (Class|BPIPickable|Launch(Message) (Variables|Default|GetactualCrate) (* (Variables|Default|GetlaunchStrength) (Math|Vector|GetForwardVector (Variables|Default|GetthrowArrow)) (Variables|/Game/_Manager/InGame/DataAsset/BP/BP_Player_DA.BP_Player_DA_C|GetlaunchingStrenghFactor (Variables|Default|GetdataAsset))))
    (Transformation|DetachFromActor (Variables|Default|GetactualCrate) "KeepWorld" "KeepWorld" "KeepWorld")
    (Variables|Default|SetactualCrate 0)
    (Utilities|FlowControl|Delay 0.4)
    (Components|Activation|SetActive (Variables|Default|GetboxDetection) true false)
    (Components|Activation|SetActive (Variables|Default|GetboxDetection1) true false)
    (Variables|Default|SetlaunchStrength 0.0)))

(event EventSteering
  (params (Force :type Float%20%28double-precision%29))
  ;[1 1 1] Move Player
  (Class|ChaosVehicleMovementComponent|SetSteeringInput (Variables|Default|GetVehicleMovementComponent) Force))

(event EventBrakeReverse
  (params (Force :type Float%20%28double-precision%29))
  (bind _vehiclemovementcomponent (Variables|Default|GetVehicleMovementComponent))
  ;[1 1 1] Move Player
  (Class|ChaosVehicleMovementComponent|SetThrottleInput _vehiclemovementcomponent 0.0)
  (Class|ChaosVehicleMovementComponent|SetBrakeInput _vehiclemovementcomponent Force))

(event EventSetRespawn
  (params (transform :type Transform))
  ;[1 1 1] Respawn
  (Variables|Default|SetcheckpointTransform transform))

(event EventRespawnActor
  ;[1 1 1] Respawn
  (Transformation|SetActorTransform (Variables|Default|GetcheckpointTransform) false true))

(event EventAccelerate
  (params (Force :type Float%20%28double-precision%29))
  (bind _vehiclemovementcomponent (Variables|Default|GetVehicleMovementComponent))
  ;[1 1 1] Move Player
  (Class|ChaosVehicleMovementComponent|SetThrottleInput _vehiclemovementcomponent Force)
  (Class|ChaosVehicleMovementComponent|SetBrakeInput _vehiclemovementcomponent 0.0))

(event EventLook
  (params (axis :type Vector%202D%20Structure))
  ;[1 1 1] Look
  (Pawn|Input|AddControllerPitchInput (.y axis))
  (Pawn|Input|AddControllerYawInput (.x axis))
  (Utilities|FlowControl|Sequence
    (:then_0
      (Utilities|FlowControl|RetriggerableDelay (Variables|/Game/_Manager/InGame/DataAsset/BP/BP_Player_DA.BP_Player_DA_C|GetcameraAutoRotTime (Variables|Default|GetdataAsset)))
      (bind _returnvalue (Utilities|Time|SetTimerbyEvent (delegate Custom|RotateCam) 0.001 true true)))
    (:then_1
      (Utilities|Time|PauseTimerbyHandle _returnvalue))))

(event EventPause
  ;[1 1 1] Pause
  (bind _ashud_game (Utilities|Casting|CastToHUD_Game (HUD|GetHUD (Game|GetPlayerController 0))))
  (bind _returnvalue (Class|CommonActivatableWidgetContainerBase|AddWidget (Variables|/Game/Blueprints/UI/WBP_BaseViewport.WBP_BaseViewport_C|GetstackWidget (Variables|/Game/_Manager/InGame/HUD_Game.HUD_Game_C|GetbaseViewportRef _ashud_game)) "/Game/Blueprints/UI/WBP_PauseMenu.WBP_PauseMenu_C"))
  (bind _output_get (Variables|Default|SetPauseMenuWidget _returnvalue))
  (Variables|/Game/Blueprints/UI/WBP_PauseMenu.WBP_PauseMenu_C|SetCamera _output_get (Variables|Default|GetCamera)))

(event EventLift
  (params (up :type Boolean))
  (bind _dataasset (Variables|Default|GetdataAsset))
  (bind _dataasset_2 (Variables|Default|GetdataAsset))
  (bind _crateloc (Variables|Default|GetCrateLoc))
  (bind _returnvalue (Transformation|GetWorldLocation _crateloc))
  ;[1 1 1] Lift Up and down
  (if up
    (bind _alpha (Timeline|forkLoc Play)
      (:Update
        (Variables|Throw|SetthrowAngle (Math|Float|Lerp (Variables|/Game/_Manager/InGame/DataAsset/BP/BP_Player_DA.BP_Player_DA_C|GetlaunchingAngleMin _dataasset) (Variables|/Game/_Manager/InGame/DataAsset/BP/BP_Player_DA.BP_Player_DA_C|GetlaunchingAngleMax _dataasset) _alpha))
        (Transformation|SetRelativeLocation (Variables|Default|GetForkLiftLift) (Math|Vector|Lerp(Vector) (Math|Vector|MakeVector 4e+01 0.0 (Variables|/Game/_Manager/InGame/DataAsset/BP/BP_Player_DA.BP_Player_DA_C|GetforkMinHeight _dataasset_2)) (Math|Vector|MakeVector 4e+01 0.0 (Variables|/Game/_Manager/InGame/DataAsset/BP/BP_Player_DA.BP_Player_DA_C|GetforkMaxHeight _dataasset_2)) _alpha) true false)
        (Transformation|SetRelativeRotation (Variables|Default|GetthrowArrow) (Math|Rotator|MakeRotator 0.0 (Variables|Throw|GetthrowAngle) 0.0) false false)
        (if (<= (Variables|/Script/Engine.ArrowComponent|GetArrowLength (Variables|Default|GetthrowArrow)) 0.01)
          (Variables|/Script/Engine.ArrowComponent|SetArrowLength (Variables|Default|GetthrowArrow) 29.5))
        (Development|SetHiddeninGame (Variables|Default|GetthrowArrow) false false)))
    (else
      (bind _returnvalue_2 (Collision|BoxTraceByChannel (- _returnvalue "0.000000,0.000000,60.000000") (- _returnvalue "0.000000,0.000000,61.000000") "50.000000,50.000000,1.000000" (Transformation|GetActorRotation) "TraceTypeQuery1" false 0 "ForOneFrame"))
      (if (not _returnvalue_2)
        (Timeline|forkLoc Reverse)
        (else
          (CallFunction|StopLift))))))

(event EventStopLift
  (bind _dataasset (Variables|Default|GetdataAsset))
  (bind _dataasset_2 (Variables|Default|GetdataAsset))
  ;[1 1 1] Lift Up and down
  (Development|SetHiddeninGame (Variables|Default|GetthrowArrow) true false)
  (bind _alpha (Timeline|forkLoc Stop)
    (:Update
      (Variables|Throw|SetthrowAngle (Math|Float|Lerp (Variables|/Game/_Manager/InGame/DataAsset/BP/BP_Player_DA.BP_Player_DA_C|GetlaunchingAngleMin _dataasset) (Variables|/Game/_Manager/InGame/DataAsset/BP/BP_Player_DA.BP_Player_DA_C|GetlaunchingAngleMax _dataasset) _alpha))
      (Transformation|SetRelativeLocation (Variables|Default|GetForkLiftLift) (Math|Vector|Lerp(Vector) (Math|Vector|MakeVector 4e+01 0.0 (Variables|/Game/_Manager/InGame/DataAsset/BP/BP_Player_DA.BP_Player_DA_C|GetforkMinHeight _dataasset_2)) (Math|Vector|MakeVector 4e+01 0.0 (Variables|/Game/_Manager/InGame/DataAsset/BP/BP_Player_DA.BP_Player_DA_C|GetforkMaxHeight _dataasset_2)) _alpha) true false)
      (Transformation|SetRelativeRotation (Variables|Default|GetthrowArrow) (Math|Rotator|MakeRotator 0.0 (Variables|Throw|GetthrowAngle) 0.0) false false)
      (if (<= (Variables|/Script/Engine.ArrowComponent|GetArrowLength (Variables|Default|GetthrowArrow)) 0.01)
        (Variables|/Script/Engine.ArrowComponent|SetArrowLength (Variables|Default|GetthrowArrow) 29.5))
      (Development|SetHiddeninGame (Variables|Default|GetthrowArrow) false false))))

(fn ConstructionScript)

(fn SetupCameraAssets
  (bind _returnvalue (Game|GetPlayerCameraManager 0))
  (bind _dataasset (Variables|Default|GetdataAsset))
  (bind _dataasset_2 (Variables|Default|GetdataAsset))
  (Variables|/Script/Engine.SpringArmComponent|SetTargetArmLength (Variables|Default|GetSpringArm) (Variables|/Game/_Manager/InGame/DataAsset/BP/BP_Player_DA.BP_Player_DA_C|GetcameraArmLength _dataasset_2))
  (Camera|SetFieldOfView (Variables|Default|GetCamera) (Variables|/Game/_Manager/InGame/DataAsset/BP/BP_Player_DA.BP_Player_DA_C|GetFOV _dataasset_2))
  (Variables|/Script/Engine.PlayerCameraManager|SetViewPitchMin _returnvalue (Variables|/Game/_Manager/InGame/DataAsset/BP/BP_Player_DA.BP_Player_DA_C|GetminCamHeight _dataasset))
  (Variables|/Script/Engine.PlayerCameraManager|SetViewPitchMax _returnvalue (Variables|/Game/_Manager/InGame/DataAsset/BP/BP_Player_DA.BP_Player_DA_C|GetmaxCamHeight _dataasset))
  (return))

(fn DesiredRotation
  (bind _returnvalue (Transformation|GetActorForwardVector))
  (bind _returnvalue_2 (Transformation|GetActorRightVector))
  (bind _returnvalue_3 (Input|EnhancedActionValues|GetIA_Steering))
  (bind _returnvalue_4 (* _returnvalue_2 _returnvalue_3 -1.0))
  (bind _returnvalue_5 (+ _returnvalue _returnvalue_4))
  (Transformation|SetWorldRotation (Variables|Default|GetInputRotation) (Math|Rotator|MakeRotfromX _returnvalue_5) false false)
  (return _returnvalue_5))

(fn SetExhaustVFX
  (params (InValue :type Boolean))
  (for _array_element (Utilities|Array|MakeArray (Variables|Default|GetNS_Exhaust2) (Variables|Default|GetNS_Exhaust1) (Variables|Default|GetNS_Exhaust) (Variables|Default|GetNS_Exhaust3))
    (Class|NiagaraComponent|SetVariableBool _array_element "Boost" InValue))
  (return))

(fn GetChargePercent
  (return (/ (Variables|Default|GetlaunchStrength) (Variables|/Game/_Manager/InGame/DataAsset/BP/BP_Player_DA.BP_Player_DA_C|GetlaunchHoldTime (Variables|Default|GetdataAsset)))))

(fn GetCrate
  (return (Variables|Default|GetactualCrate)))