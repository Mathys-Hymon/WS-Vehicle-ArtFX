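; Actor component that auto-respawns a Chaos wheeled vehicle when its wheels lose ground contact for too long.
; A looping timer drives a check of the four wheels' contact states, counting those in the air.
; Fewer than two airborne saves the location as valid; otherwise consecutive failures accumulate.
; At the failure threshold, the vehicle teleports to the last valid location, keeping only its yaw so it lands upright.
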(event Custom|CheckValidPosition
  ;[1 1 1] Check how many wheels touch the floor
  (bind _fyingwheels (CallFunction|FlyingWheelsCount (CallFunction|WheelsontheFloor)))
  (if (>= _fyingwheels 2)
    ;[1 1 1] increment invalid check, if greater or equal to check amount respawn the vehicle and reset invalid check count
    (bind _result (Math|Integer|IncrementInt (Variables|Local|GetInvalidCheckCount))
      (:%20%20
        (if (>= _result (Variables|AutoRespawn|GetInvalidCheckAmount))
          (CallFunction|RespawnVehicle)
          (Variables|Local|SetInvalidCheckCount 0))))
    (else
      ;[1 1 1] Reset invalid count and set the last valid location
      (Variables|Local|SetInvalidCheckCount 0)
      (Variables|Local|SetLastValidLocation (Transformation|GetActorLocation (Components|GetOwner))))))

(event Custom|RespawnVehicle
  ;[1 1 1] RespawnVehicle
  (Transformation|SetActorTransform (Components|GetOwner) (Math|Transform|MakeTransform (Variables|Local|GetLastValidLocation) (Math|Rotator|MakeRotator 0.0 0.0 (.yaw (Transformation|GetActorRotation (Components|GetOwner))))) false true))

(event EventBeginPlay
  (bind _output_get (Variables|Local|Component|SetMovementsComponent (Actor|GetComponentbyClass (Components|GetOwner) "/Script/ChaosVehicles.ChaosVehicleMovementComponent")))
  (bind _aschaos_wheeled_vehicle_movement_component (Utilities|Casting|CastToChaosWheeledVehicleMovementComponent _output_get))
  (Variables|Local|Component|SetWheeledComponent _aschaos_wheeled_vehicle_movement_component)
  (Utilities|Time|SetTimerbyEvent (EventDispatchers|CreateEvent :!event Custom|CheckValidPosition) (Variables|AutoRespawn|GetCheckValidityDelay) true))

(fn WheelsontheFloor
  (bind _wheeledcomponent (Variables|Local|Component|GetWheeledComponent))
  (for _array_element (Utilities|Array|MakeArray (Class|ChaosWheeledVehicleMovementComponent|GetWheelState _wheeledcomponent) (Class|ChaosWheeledVehicleMovementComponent|GetWheelState _wheeledcomponent 1) (Class|ChaosWheeledVehicleMovementComponent|GetWheelState _wheeledcomponent 2) (Class|ChaosWheeledVehicleMovementComponent|GetWheelState _wheeledcomponent 3))
    (Utilities|Array|Add (LocalVariables|GetWheelsOnTheFloor) (.bInContact (Class|ChaosWheeledVehicleMovementComponent|BreakWheelStatus _array_element))))
  (return (LocalVariables|GetWheelsOnTheFloor)))

(fn FlyingWheelsCount
  (params (bValue :type Array%20of%20Booleans))
  (for _array_element bValue
    (if (not _array_element)
      (LocalVariables|SetOnAirCount (+ (LocalVariables|GetOnAirCount) 1))))
  (return (LocalVariables|GetOnAirCount)))