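; Pause-menu forklift actor that slides horizontally on and off screen relative to the camera.
; EnterScreen and GoOffScreen set a flag, reset the timer and store the start location.
; Tick offsets it along the camera's right vector and calls ForkliftInPlace when the timer reaches one.
; The exit branch adds zero to the timer and clears only the enter flag, so as written it never completes.
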(event Custom|GoOffScreen
  (Variables|Default|SetCanGoOfScreen true)
  (Variables|Default|SetDeltaSeconds 0.0)
  (Variables|Default|SetBaseActorLocation (Transformation|GetActorLocation)))

(event Custom|EnterScreen
  (Variables|Default|SetCanEnterScreen true)
  (Variables|Default|SetDeltaSeconds 0.0)
  (Variables|Default|SetBaseActorLocation (Transformation|GetActorLocation)))

(event EventTick
  (params (DeltaSeconds :type Float%20%28single-precision%29))
  (if (Variables|Default|GetCanEnterScreen)
    (Variables|Default|SetDeltaSeconds (+ (Variables|Default|GetDeltaSeconds) DeltaSeconds))
    (Transformation|SetActorLocation (- (Variables|Default|GetBaseActorLocation) (* (Math|Vector|GetRightVector (Variables|Default|GetCamera)) (* (Variables|Default|GetDeltaSeconds) 4e+02))) false false)
    (if (>= (Variables|Default|GetDeltaSeconds) 1.0)
      (Variables|Default|SetCanEnterScreen false)
      (Transformation|SetActorLocation (- (Variables|Default|GetBaseActorLocation) (* (Math|Vector|GetRightVector (Variables|Default|GetCamera)) 4e+02)) false false)
      (Default|CallForkliftinPlace :!label _label))
    (elif (Variables|Default|GetCanGoOfScreen)
      (Variables|Default|SetDeltaSeconds (+ (Variables|Default|GetDeltaSeconds) 0.0))
      (Transformation|SetActorLocation (+ (Variables|Default|GetBaseActorLocation) (* (Math|Vector|GetRightVector (Variables|Default|GetCamera)) (* (Variables|Default|GetDeltaSeconds) 4e+02))) false false)
      (if (>= (Variables|Default|GetDeltaSeconds) 1.0)
        (Variables|Default|SetCanEnterScreen false)
        (Transformation|SetActorLocation (+ (Variables|Default|GetBaseActorLocation) (* (Math|Vector|GetRightVector (Variables|Default|GetCamera)) 4e+02)) false false)
        (goto _label)))))

(fn ConstructionScript)