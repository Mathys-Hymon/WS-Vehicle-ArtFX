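; Pause menu settings box actor that slides on and off screen to show or hide the settings menu.
; EnterScreen caches the actor's Y position and plays a Timeline that offsets it along Y, while GoOffScreen reverses that Timeline from the end.
; When the Timeline finishes, the CanOpenSettings flag ensures ShowSettingMenu is called only after entering, not after leaving.
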(event Custom|GoOffScreen
  (bind _returnvalue (Transformation|GetActorLocation))
  ;[1 1 1] show or hide Setting menu
  (Variables|Default|SetcanOpenSettings false)
  (bind _newtrack_0 (Timeline|Timeline ReverseFromEnd)
    (:Update
      (Transformation|SetActorLocation (Math|Vector|MakeVector (.x _returnvalue) (+ _newtrack_0 (Variables|Default|GetReturn%20Value%20Y)) (.z _returnvalue)) false false))
    (:Finished
      (if (Variables|Default|GetcanOpenSettings)
        (Default|CallShowSettingMenu)))))

(event Custom|EnterScreen
  (bind _returnvalue (Transformation|GetActorLocation))
  ;[1 1 1] show or hide Setting menu
  (Variables|Default|SetcanOpenSettings true)
  (Variables|Default|SetReturn%20Value%20Y (.y (Transformation|GetActorLocation)))
  (bind _newtrack_0 (Timeline|Timeline Play)
    (:Update
      (Transformation|SetActorLocation (Math|Vector|MakeVector (.x _returnvalue) (+ _newtrack_0 (Variables|Default|GetReturn%20Value%20Y)) (.z _returnvalue)) false false))
    (:Finished
      (if (Variables|Default|GetcanOpenSettings)
        (Default|CallShowSettingMenu)))))

(fn ConstructionScript)