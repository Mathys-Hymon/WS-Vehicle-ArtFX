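; BP_LevelBox is a menu actor that slides on and off screen and signals when the level menu can show.
; EnterScreen stores its current Y, then plays a Timeline that offsets the actor along Y from that value.
; GoOffScreen reverses the same Timeline from the end.
; A CanOpenLevels flag ensures the ShowLevelMenu call fires only when the entering slide finishes, not the exit.
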(event Custom|GoOffScreen
  (bind _returnvalue (Transformation|GetActorLocation))
  ;[1 1 1] show or hide Setting menu
  (Variables|Default|SetcanOpenLevels false)
  (bind _newtrack_0 (Timeline|Timeline ReverseFromEnd)
    (:Update
      (Transformation|SetActorLocation (Math|Vector|MakeVector (.x _returnvalue) (+ _newtrack_0 (Variables|Default|GetReturn%20Value%20Y)) (.z _returnvalue)) false false))
    (:Finished
      (if (Variables|Default|GetcanOpenLevels)
        (Default|CallShowLevelMenu)))))

(event Custom|EnterScreen
  (bind _returnvalue (Transformation|GetActorLocation))
  ;[1 1 1] show or hide Setting menu
  (Variables|Default|SetcanOpenLevels true)
  (Variables|Default|SetReturn%20Value%20Y (.y (Transformation|GetActorLocation)))
  (bind _newtrack_0 (Timeline|Timeline Play)
    (:Update
      (Transformation|SetActorLocation (Math|Vector|MakeVector (.x _returnvalue) (+ _newtrack_0 (Variables|Default|GetReturn%20Value%20Y)) (.z _returnvalue)) false false))
    (:Finished
      (if (Variables|Default|GetcanOpenLevels)
        (Default|CallShowLevelMenu)))))

(fn ConstructionScript)