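; Main menu box actor that slides along world Y to move between the main menu, the settings (right) and the levels (left).
; Each Go event caches the current Y and plays its own timeline, whose track is added as an offset to that cached value.
; The Reverse events play that timeline back from the end and set CanOpenMenu, so CallShowMenuWidget fires only when the return slide finishes.
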(event Custom|ReverseLeft
  (bind _returnvalue (Transformation|GetActorLocation))
  ;[1 1 1] Go to the levels
  (Variables|Default|SetcanOpenMenu true)
  (bind _newtrack_0 (Timeline|Timeline ReverseFromEnd)
    (:Update
      (Transformation|SetActorLocation (Math|Vector|MakeVector (.x _returnvalue) (+ _newtrack_0 (Variables|Default|GetyValue)) (.z _returnvalue)) false false))
    (:Finished
      (if (Variables|Default|GetcanOpenMenu)
        (Default|CallShowMenuWidget)))))

(event Custom|GoRight
  (bind _returnvalue (Transformation|GetActorLocation))
  ;[1 1 1] Go to the setting
  (Variables|Default|SetcanOpenMenu false)
  (Variables|Default|SetyValue (.y (Transformation|GetActorLocation)))
  (bind _newtrack_0 (Timeline|Move Play)
    (:Update
      (Transformation|SetActorLocation (Math|Vector|MakeVector (.x _returnvalue) (+ _newtrack_0 (Variables|Default|GetyValue)) (.z _returnvalue)) false false))
    (:Finished
      (if (Variables|Default|GetcanOpenMenu)
        (Default|CallShowMenuWidget)))))

(event Custom|GoLeft
  (bind _returnvalue (Transformation|GetActorLocation))
  ;[1 1 1] Go to the levels
  (Variables|Default|SetcanOpenMenu false)
  (Variables|Default|SetyValue (.y (Transformation|GetActorLocation)))
  (bind _newtrack_0 (Timeline|Timeline Play)
    (:Update
      (Transformation|SetActorLocation (Math|Vector|MakeVector (.x _returnvalue) (+ _newtrack_0 (Variables|Default|GetyValue)) (.z _returnvalue)) false false))
    (:Finished
      (if (Variables|Default|GetcanOpenMenu)
        (Default|CallShowMenuWidget)))))

(event Custom|ReverseRight
  (bind _returnvalue (Transformation|GetActorLocation))
  ;[1 1 1] Go to the setting
  (Variables|Default|SetcanOpenMenu true)
  (bind _newtrack_0 (Timeline|Move ReverseFromEnd)
    (:Update
      (Transformation|SetActorLocation (Math|Vector|MakeVector (.x _returnvalue) (+ _newtrack_0 (Variables|Default|GetyValue)) (.z _returnvalue)) false false))
    (:Finished
      (if (Variables|Default|GetcanOpenMenu)
        (Default|CallShowMenuWidget)))))

(fn ConstructionScript)