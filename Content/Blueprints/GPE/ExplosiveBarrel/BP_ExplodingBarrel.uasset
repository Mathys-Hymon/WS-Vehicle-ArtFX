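; BP_ExplodingBarrel is a launchable physics barrel that explodes once on hard impacts with anything but the player pawn.
; After a short random delay, it spawns VFX and a rumble emitter, plays sound and camera shake, then sphere-traces its data-asset radius.
; Hit barrels chain-react through BPI_ExplodingBarrel, while other actors receive force through BPI_ExplosionReaction components.
; From inside that hit loop, it notifies its Dispenser and destroys itself a tick later.
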(event OnComponentHit(BarrelMesh)
  (params (HitComponent :type Primitive%20Component%20Object%20Reference) (OtherActor :type Actor%20Object%20Reference) (OtherComp :type Primitive%20Component%20Object%20Reference) (NormalImpulse :type Vector :default "0, 0, 0") (Hit :type Hit%20Result%20Structure%20%28by%20ref%29))
  ;[1 1 1] Check if it has to explode
  (if (and (< (Variables|/Game/_Manager/InGame/DataAsset/BP/BP_ExplosiveCrates_DA.BP_ExplosiveCrates_DA_C|GetexplosionSensivity (Variables|Default|GetexplosiveCrateDA)) (+ (Math|Vector|VectorLength (Transformation|GetVelocity)) (Math|Vector|VectorLength (Transformation|GetComponentVelocity (Variables|Default|GetBarrelMesh))))) (not (== OtherActor (Game|Player|GetPlayerPawn 0))))
    (CallFunction|TakeDamages)))

(event EventSwitchHitSimulation
  (params (bool :type Boolean))
  (Class|PrimitiveComponent|SetNotifyRigidBodyCollision (Variables|Default|GetBarrelMesh) bool))

(event EventLaunch
  (params (direction :type Vector :default "0, 0, 0"))
  ;[1 1 1] LaunchCrate
  (CallFunction|ChangePhysic true self)
  (Physics|AddImpulse (Variables|Default|GetBarrelMesh) (* direction 1e+02) "None" true)
  ;;[0.1246 0.6719 0] Sound
  (Audio|PlaySoundatLocation (Variables|/Game/Imports/SFX/Sounds/BPA_SFX.BPA_SFX_C|GetLaunchBoxBoing (Variables|Default|GetSFXDatas)) (Transformation|GetActorLocation) "0, 0, 0" 1.0 1.0 0.0 0 0 0 0))

(event EventChangePhysic
  (params (enable :type Boolean) (parent :type Actor%20Object%20Reference))
  ;[1 1 1] Change physic
  (Physics|SetSimulatePhysics (Variables|Default|GetBarrelMesh) enable)
  (Variables|Default|SetParent parent)
  (Collision|SetCollisionResponsetoChannel (Variables|Default|GetBarrelMesh) "ECC_GameTraceChannel1" (select enable "ECR_Block" "ECR_Ignore")))

(event EventTakeDamages
  (bind _explosivecrateda (Variables|Default|GetexplosiveCrateDA))
  (bind _barrelmesh (Variables|Default|GetBarrelMesh))
  (bind _explosivecrateda_2 (Variables|Default|GetexplosiveCrateDA))
  (bind _returnvalue (Transformation|GetWorldLocation _barrelmesh))
  (bind _explosionradius (Variables|/Game/_Manager/InGame/DataAsset/BP/BP_ExplosiveCrates_DA.BP_ExplosiveCrates_DA_C|GetexplosionRadius _explosivecrateda))
  ;[1 1 1] If The life is < 0, the barrel Explodes
  (Utilities|FlowControl|DoOnce false
    (:Completed
      (Utilities|FlowControl|Delay (Math|Random|RandomFloatinRange 0.2 0.6))
      (Game|SpawnActorfromClass "/Game/Blueprints/GamepadRumble/BP_ExplosionRumbleEmetor.BP_ExplosionRumbleEmetor_C" (Transformation|GetActorTransform) "Undefined" "MultiplyWithRoot" 0 0)
      ;;[1 0 0] VFX
      (Game|SpawnActorfromClass "/Game/Blueprints/GPE/ExplosiveBarrel/Explosion/BP_Explosion.BP_Explosion_C" (Math|Transform|MakeTransform (Transformation|GetActorLocation) "0, 0, 0" "1.000000,1.000000,1.000000") "Undefined" "MultiplyWithRoot" 0 0)
      ;;[0.1246 0.6719 0] Sound
      (Audio|PlaySoundatLocation (Variables|/Game/Imports/SFX/Sounds/BPA_SFX.BPA_SFX_C|GetFireworkExplosion (Variables|Default|GetSFXDatas)) _returnvalue "0, 0, 0" 1.0 1.0 0.0 0 0 0 0)
      (Camera|PlayWorldCameraShake "/Game/Blueprints/CameraShake/BP_ExplosionBarrelCameraShake.BP_ExplosionBarrelCameraShake_C" _returnvalue _explosionradius _explosionradius)
      (bind _outhits (Collision|MultiSphereTraceByChannel _returnvalue _returnvalue _explosionradius "TraceTypeQuery1" false 0 "None"))
      (for _array_element _outhits
        (Utilities|IsValid (.HitActor (Collision|BreakHitResult _array_element))
          (:Is%20Valid
            (if (Utilities|DoesObjectImplementInterface (.HitActor (Collision|BreakHitResult _array_element)) "/Game/Blueprints/BPI/BPI_ExplodingBarrel.BPI_ExplodingBarrel_C")
              (Class|BPIExplodingBarrel|TakeDamages(Message) (.HitActor (Collision|BreakHitResult _array_element)))
              (else
                (Class|BPIExplosionReaction|Explodes(Message) (Utilities|Array|Get(acopy) (Class|Actor|GetComponentsbyInterface (.HitActor (Collision|BreakHitResult _array_element)) "/Game/Blueprints/BPI/BPI_ExplosionReaction.BPI_ExplosionReaction_C")) (Transformation|GetActorLocation) (Variables|/Game/_Manager/InGame/DataAsset/BP/BP_ExplosiveCrates_DA.BP_ExplosiveCrates_DA_C|GetexplosinForce _explosivecrateda_2) (Variables|/Game/_Manager/InGame/DataAsset/BP/BP_ExplosiveCrates_DA.BP_ExplosiveCrates_DA_C|GetexplosionRadius _explosivecrateda_2))))
            (Utilities|FlowControl|DelayUntilNextTick)
            (Utilities|IsValid (Variables|Default|GetDispenser)
              (:Is%20Valid
                (Default|CallBarrelExploded (Variables|Default|GetDispenser)))
              (:Is%20Not%20Valid
                _))
            (Actor|DestroyActor)))))))

(fn ConstructionScript)