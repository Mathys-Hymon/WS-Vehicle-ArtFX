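; Dispenser actor that keeps an exploding barrel available in the level by respawning it after it explodes.
; On BeginPlay it spawns a BP_ExplodingBarrel at its own transform, offset along world X, and passes itself as the barrel's Dispenser.
; It binds to the barrel's exploded event, which waits a configurable delay before spawning and binding the next barrel, forming an event-driven loop without Tick.
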(event Custom|SpawnNewBarrel
  (Utilities|FlowControl|Delay (Variables|Default|GetDelayBeforeSpawn))
  (CallFunction|SpawnBarrel))

(event Custom|SpawnBarrel
  (bind _returnvalue (Transformation|GetActorTransform))
  (Game|SpawnActorfromClass "/Game/Blueprints/GPE/ExplosiveBarrel/BP_ExplodingBarrel.BP_ExplodingBarrel_C" (Math|Transform|MakeTransform (Math|Vector|MakeVector (+ (.x (.location _returnvalue)) (Variables|Default|GetSpawnOffset)) (.y (.location _returnvalue)) (.z (.location _returnvalue))) (.rotation _returnvalue) "1.000000,1.000000,1.000000") "Undefined" "MultiplyWithRoot" 0 self 0)
  (EventDispatchers|BindEventtoBarrelExploded (delegate Custom|SpawnNewBarrel)))

(event EventBeginPlay
  (bind _returnvalue (Transformation|GetActorTransform))
  (Game|SpawnActorfromClass "/Game/Blueprints/GPE/ExplosiveBarrel/BP_ExplodingBarrel.BP_ExplodingBarrel_C" (Math|Transform|MakeTransform (Math|Vector|MakeVector (+ (.x (.location _returnvalue)) (Variables|Default|GetSpawnOffset)) (.y (.location _returnvalue)) (.z (.location _returnvalue))) (.rotation _returnvalue) "1.000000,1.000000,1.000000") "Undefined" "MultiplyWithRoot" 0 self 0)
  (EventDispatchers|BindEventtoBarrelExploded (delegate Custom|SpawnNewBarrel)))

(event Collision|EventActorBeginOverlap
  (params (OtherActor :type Actor%20Object%20Reference)))

(event EventTick
  (params (DeltaSeconds :type Float%20%28single-precision%29)))

(fn ConstructionScript)