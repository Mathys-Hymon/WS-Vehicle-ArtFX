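; Physics crate prop with configurable mesh, material and mass that plays a cardboard box sound when it hits something.
; BeginPlay enables physics and starts a four-second timer, while a CanMakeNoise flag gates impact sounds.
; Hits spawn the cue at the impact point, passing an inversely mapped actor speed as its Power parameter.
; A DoOnce with a short randomized delayed reset throttles repeated sounds.
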(event OnComponentHit(SM_Prop_Crate_03)
  (params (HitComponent :type Primitive%20Component%20Object%20Reference) (OtherActor :type Actor%20Object%20Reference) (OtherComp :type Primitive%20Component%20Object%20Reference) (NormalImpulse :type Vector :default "0, 0, 0") (Hit :type Hit%20Result%20Structure%20%28by%20ref%29))
  (if (Variables|Default|GetbCanMakeNoise)
    (Utilities|FlowControl|Sequence
      (:then_0
        (Utilities|FlowControl|DoOnce false :!label _label
          (:Completed
            (bind _returnvalue (Audio|SpawnSoundatLocation "/Game/Imports/SFX/Sounds/Crate/Cue_CardBox.Cue_CardBox" (.Location (Collision|BreakHitResult Hit)) "0, 0, 0" 0.6 1.0 0.0 0 0))
            (Effects|Components|ParticleSystem|SetIntParameter _returnvalue "Power" (Math|Float|Truncate (Math|Float|MapRangeClamped (Math|Vector|VectorLength (Transformation|GetVelocity)) 5e+02 3e+01 0.0 5.0))))))
      (:then_1
        (Utilities|FlowControl|Delay (Math|Random|RandomFloatinRange 0.4 0.6))
        (goto _label Reset)))))

(event Custom|StartMakingNoise
  (Variables|Default|SetbCanMakeNoise true))

(event EventBeginPlay
  (Class|PrimitiveComponent|SetAllMassScale (Variables|Default|GetSM_Prop_Crate_03) (Variables|Default|GetMass))
  (Physics|SetSimulatePhysics (Variables|Default|GetSM_Prop_Crate_03) true)
  (Utilities|Time|SetTimerbyEvent (EventDispatchers|CreateEvent :!event Custom|StartMakingNoise) 4.0))

(fn ConstructionScript
  (Components|StaticMesh|SetStaticMesh (Variables|Default|GetSM_Prop_Crate_03) (Variables|Default|GetMesh))
  (Rendering|Material|SetMaterial (Variables|Default|GetSM_Prop_Crate_03) 0 (Variables|Default|GetMaterial)))