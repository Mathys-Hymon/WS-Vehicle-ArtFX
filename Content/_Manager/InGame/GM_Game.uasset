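; GM_Game is the in-game manager that tracks box organisation progress and detects when a level is complete.
; SetBoxAmount increments the total box count by one per call.
; CheckBoxOrganization compares OrganizedBoxes, which this graph never modifies, against that total and prints either a completion or keep-going message with the organised count.
; Completion is only debug text so far, with a comment marking where the level-complete sound belongs.
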(event Custom|CheckBoxOrganization
  (bind _organizedboxes (Variables|Default|GetOrganizedBoxes))
  ;[1 1 1] Check if all boxes in the level have been organised
  (if (== (Variables|Default|GetOrganizedBoxes) (Variables|Default|GetBoxes))
    ;;[1 0 0] Lvl complete sound here
    (Development|PrintString "Level Complete!!")
    (Development|PrintString (Utilities|String|ToString(Integer) _organizedboxes))
    (else
      (Development|PrintString "Keep going!")
      (Development|PrintString (Utilities|String|ToString(Integer) _organizedboxes)))))

(event Custom|SetBoxAmount
  ;[1 1 1] Increment the amount of boxes to keep track of
  (bind _result (Math|Integer|IncrementInt (Variables|Default|GetBoxes))
    (:%20%20
      (bind _output_get (Variables|Default|SetBoxes _result)))))

(fn ConstructionScript)