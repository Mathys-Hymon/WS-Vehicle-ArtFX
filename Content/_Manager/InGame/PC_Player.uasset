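; Player controller that adds the player Enhanced Input mapping context on BeginPlay and relays input as messages.
; Driving, look, boost, lift and box-throw inputs go to the controlled pawn, while interact targets player character 0 and pause targets player pawn 0.
; Driving axes forward on both Triggered and Completed, lift sends a stop on release, and box throw uses hold time to charge and launch.
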(event Input|EnhancedActionEvents|EnhancedInputActionIA_Look
  (params (ActionValue :type Vector%202D%20Structure) (ElapsedSeconds :type Float%20%28double-precision%29) (TriggeredSeconds :type Float%20%28double-precision%29) (InputAction :type Input%20Action%20Object%20Reference :default "/Game/_Manager/Inputs/Player/IA/IA_Look.IA_Look"))
  ;[1 1 1] Look
  (Class|BPIPlayer|Look(Message) (Pawn|GetControlledPawn) ActionValue))

(event Input|EnhancedActionEvents|EnhancedInputActionIA_Accelerator
  (params (ActionValue :type Float%20%28double-precision%29) (ElapsedSeconds :type Float%20%28double-precision%29) (TriggeredSeconds :type Float%20%28double-precision%29) (InputAction :type Input%20Action%20Object%20Reference :default "/Game/_Manager/Inputs/Player/IA/IA_Accelerator.IA_Accelerator"))
  ;[1 1 1] Move
  (:Triggered
    (Class|BPIPlayer|Accelerate(Message) (Pawn|GetControlledPawn) ActionValue :!label _label))
  (:Completed
    (goto _label)))

(event Input|EnhancedActionEvents|EnhancedInputActionIA_Brake-Reverse
  (params (ActionValue :type Float%20%28double-precision%29) (ElapsedSeconds :type Float%20%28double-precision%29) (TriggeredSeconds :type Float%20%28double-precision%29) (InputAction :type Input%20Action%20Object%20Reference :default "/Game/_Manager/Inputs/Player/IA/IA_Brake-Reverse.IA_Brake-Reverse"))
  ;[1 1 1] Brake/Reverse
  (:Triggered
    (Class|BPIPlayer|BrakeReverse(Message) (Pawn|GetControlledPawn) ActionValue :!label _label))
  (:Completed
    (goto _label)))

(event Input|EnhancedActionEvents|EnhancedInputActionIA_Steering
  (params (ActionValue :type Float%20%28double-precision%29) (ElapsedSeconds :type Float%20%28double-precision%29) (TriggeredSeconds :type Float%20%28double-precision%29) (InputAction :type Input%20Action%20Object%20Reference :default "/Game/_Manager/Inputs/Player/IA/IA_Steering.IA_Steering"))
  ;[1 1 1] Steering
  (:Triggered
    (Class|BPIPlayer|Steering(Message) (Pawn|GetControlledPawn) ActionValue :!label _label))
  (:Completed
    (goto _label)))

(event Input|EnhancedActionEvents|EnhancedInputActionIA_Interract
  (params (ActionValue :type Boolean) (ElapsedSeconds :type Float%20%28double-precision%29) (TriggeredSeconds :type Float%20%28double-precision%29) (InputAction :type Input%20Action%20Object%20Reference :default "/Game/_Manager/Inputs/Player/IA/IA_Interract.IA_Interract"))
  ;[1 1 1] Interract
  (:Started
    (Class|BPIPlayer|Interract(Message) (Game|GetPlayerCharacter 0))))

(event Input|EnhancedActionEvents|EnhancedInputActionIA_Pause
  (params (ActionValue :type Boolean) (ElapsedSeconds :type Float%20%28double-precision%29) (TriggeredSeconds :type Float%20%28double-precision%29) (InputAction :type Input%20Action%20Object%20Reference :default "/Game/_Manager/Inputs/Player/IA/IA_Pause.IA_Pause"))
  ;[1 1 1] Pause
  (:Started
    (Class|BPIPlayer|Pause(Message) (Game|Player|GetPlayerPawn 0))))

(event Input|EnhancedActionEvents|EnhancedInputActionIA_LiftUp
  (params (ActionValue :type Boolean) (ElapsedSeconds :type Float%20%28double-precision%29) (TriggeredSeconds :type Float%20%28double-precision%29) (InputAction :type Input%20Action%20Object%20Reference :default "/Game/_Manager/Inputs/Player/IA/IA_LiftUp.IA_LiftUp"))
  (bind _returnvalue (Pawn|GetControlledPawn))
  ;[1 1 1] Lift
  (:Started
    (Class|BPIPlayer|Lift(Message) _returnvalue true))
  (:Completed
    (Class|BPIPlayer|StopLift(Message) _returnvalue)))

(event Input|EnhancedActionEvents|EnhancedInputActionIA_LiftDown
  (params (ActionValue :type Boolean) (ElapsedSeconds :type Float%20%28double-precision%29) (TriggeredSeconds :type Float%20%28double-precision%29) (InputAction :type Input%20Action%20Object%20Reference :default "/Game/_Manager/Inputs/Player/IA/IA_LiftDown.IA_LiftDown"))
  (bind _returnvalue (Pawn|GetControlledPawn))
  ;[1 1 1] Lift
  (:Triggered
    (Class|BPIPlayer|Lift(Message) _returnvalue false))
  (:Completed
    (Class|BPIPlayer|StopLift(Message) _returnvalue)))

(event Input|EnhancedActionEvents|EnhancedInputActionIA_ThrowBox
  (params (ActionValue :type Boolean) (ElapsedSeconds :type Float%20%28double-precision%29) (TriggeredSeconds :type Float%20%28double-precision%29) (InputAction :type Input%20Action%20Object%20Reference :default "/Game/_Manager/Inputs/Player/IA/IA_ThrowBox.IA_ThrowBox"))
  (bind _returnvalue (Pawn|GetControlledPawn))
  ;[1 1 1] ThrowBox
  (:Triggered
    (Class|BPIPlayer|ChargeBox(Message) _returnvalue ElapsedSeconds))
  (:Completed
    (Class|BPIPlayer|LaunchBox(Message) _returnvalue ElapsedSeconds)))

(event Input|EnhancedActionEvents|EnhancedInputActionIA_Boost
  (params (ActionValue :type Boolean) (ElapsedSeconds :type Float%20%28double-precision%29) (TriggeredSeconds :type Float%20%28double-precision%29) (InputAction :type Input%20Action%20Object%20Reference :default "/Game/_Manager/Inputs/Player/IA/IA_Boost.IA_Boost"))
  ;[1 1 1] Boost
  (Class|BPIPlayer|Boost(Message) (Pawn|GetControlledPawn)))

(event EventBeginPlay
  (bind _returnvalue (PlayerController|LocalPlayerSubsystems|GetEnhancedInputLocalPlayerSubsystem))
  ;[1 0 0] Add mapping Context
  (Utilities|IsValid _returnvalue
    (:Is%20Valid
      (Input|AddMappingContext _returnvalue "/Game/_Manager/Inputs/Player/IMC_Player.IMC_Player" 0 "(bIgnoreAllPressedKeysUntilRelease=True,bForceImmediately=False,bNotifyUserSettings=False)"))))

(fn ConstructionScript)